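; Parent Blueprint for casino machines that boost a player stat on interaction, with confetti and sound.
; BeginPlay rolls a random rarity, which scales the percentage-based stat gain along with a random multiplier.
; UseMachine raises Cost, re-enables the machine and optionally destroys it.
; Interact passes a zero percentage by default, and its cost check and deduction are disconnected, so use is free.
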(event Custom|UseMachine
  (params (playerRef :type BP%20First%20Person%20Character%20Object%20Reference) (addedPercent :type Float%20%28double-precision%29) (stats :type E_Stats%20Enum :default "NewEnumerator0"))
  (Niagara|SpawnSystematLocation "/Game/GAME_Casino/Folder_Adrien/NS_Confetti.NS_Confetti" (Transformation|GetActorLocation playerRef))
  (Audio|PlaySound2D "/Game/GAME_Casino/Folder_Adrien/ImportSon/Confettis/ConfettisClue.ConfettisClue" 1.0 1.0 0.0 0 0)
  (bind _value (Default|GetStats playerRef stats))
  (bind _newvalue (CallFunction|ChangeonRarity (/ (* _value addedPercent) 1e+02)))
  (Default|AddStats playerRef stats _newvalue)
  (Variables|Default|Setcost (* (Variables|Default|Getcost) 1.5))
  (Variables|Default|SetcanBeUsed? true)
  (if (Variables|Default|Getdestroy?)
    (Actor|DestroyActor)))

(event EventBeginPlay
  ;[0.15 0.15 0.15 0.5] Prendre de l'argent
  (CallFunction|SetRarity))

(event EventInteract
  (params (playerRef :type BP%20First%20Person%20Character%20Object%20Reference))
  (if (Variables|Default|GetcanBeUsed?)
    (Variables|Default|SetcanBeUsed? false)
    (Development|PrintString "INTERACT MACHINE")
    (CallFunction|UseMachine playerRef 0.0 "NewEnumerator0")
    (else
      (Audio|PlaySound2D "/Game/GAME_Casino/Folder_Adrien/ImportSon/Uhunh/UhunClue.UhunClue" 1.0 1.0 0.0 0 0))))

(fn ConstructionScript)

(fn SetRarity
  (Variables|Default|SetcurrentRarity (Utilities|Enum|ByteToEnumE_Rarity (Math|Conversions|ToByte(Integer) (Math|Random|RandomIntegerinRange 0 5)))))

(fn ChangeonRarity
  (params (value :type Float%20%28double-precision%29))
  (return (* value (* (+ (Math|Conversions|ToInteger(Byte) (Variables|Default|GetcurrentRarity)) 1) (Math|Random|RandomFloatinRange 1.0 1.5)))))

(fn ResetGold
  (Variables|Default|Setcost 32.0))