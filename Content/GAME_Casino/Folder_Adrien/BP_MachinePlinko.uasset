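; Plinko casino machine that gambles the player's stats on where a ball lands.
; Using it spawns a BP_PlinkoBall at a random Y between two local spawn limits, transformed to world space.
; Reward zones detect the "PB" tag and set a percentage Multiplier, which can be negative and doesn't always match the component name.
; ApplyReward adds that percentage of a random GambledStats stat to the player, then calls the parent's UseMachine.
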(event OnComponentBeginOverlap(Reward0.7)
  (params (OverlappedComponent :type Primitive%20Component%20Object%20Reference) (OtherActor :type Actor%20Object%20Reference) (OtherComp :type Primitive%20Component%20Object%20Reference) (OtherBodyIndex :type Integer) (bFromSweep :type Boolean) (SweepResult :type Hit%20Result%20Structure%20%28by%20ref%29))
  (if (Actor|ActorHasTag OtherActor "PB")
    (Variables|Default|Setmultiplier -3.0)
    (CallFunction|ApplyReward)))

(event OnComponentBeginOverlap(Reward0.9_2)
  (params (OverlappedComponent :type Primitive%20Component%20Object%20Reference) (OtherActor :type Actor%20Object%20Reference) (OtherComp :type Primitive%20Component%20Object%20Reference) (OtherBodyIndex :type Integer) (bFromSweep :type Boolean) (SweepResult :type Hit%20Result%20Structure%20%28by%20ref%29))
  (if (Actor|ActorHasTag OtherActor "PB")
    (Variables|Default|Setmultiplier -0.7)
    (CallFunction|ApplyReward)))

(event OnComponentBeginOverlap(Reward_3_1)
  (params (OverlappedComponent :type Primitive%20Component%20Object%20Reference) (OtherActor :type Actor%20Object%20Reference) (OtherComp :type Primitive%20Component%20Object%20Reference) (OtherBodyIndex :type Integer) (bFromSweep :type Boolean) (SweepResult :type Hit%20Result%20Structure%20%28by%20ref%29))
  (if (Actor|ActorHasTag OtherActor "PB")
    (Variables|Default|Setmultiplier 2.9)
    (CallFunction|ApplyReward)))

(event OnComponentBeginOverlap(Reward3_2)
  (params (OverlappedComponent :type Primitive%20Component%20Object%20Reference) (OtherActor :type Actor%20Object%20Reference) (OtherComp :type Primitive%20Component%20Object%20Reference) (OtherBodyIndex :type Integer) (bFromSweep :type Boolean) (SweepResult :type Hit%20Result%20Structure%20%28by%20ref%29))
  (if (Actor|ActorHasTag OtherActor "PB")
    (Variables|Default|Setmultiplier 2.9)
    (CallFunction|ApplyReward)))

(event OnComponentBeginOverlap(Reward0.9_1)
  (params (OverlappedComponent :type Primitive%20Component%20Object%20Reference) (OtherActor :type Actor%20Object%20Reference) (OtherComp :type Primitive%20Component%20Object%20Reference) (OtherBodyIndex :type Integer) (bFromSweep :type Boolean) (SweepResult :type Hit%20Result%20Structure%20%28by%20ref%29))
  (if (Actor|ActorHasTag OtherActor "PB")
    (Variables|Default|Setmultiplier -0.7)
    (CallFunction|ApplyReward)))

(event OnComponentBeginOverlap(Reward1.2_1)
  (params (OverlappedComponent :type Primitive%20Component%20Object%20Reference) (OtherActor :type Actor%20Object%20Reference) (OtherComp :type Primitive%20Component%20Object%20Reference) (OtherBodyIndex :type Integer) (bFromSweep :type Boolean) (SweepResult :type Hit%20Result%20Structure%20%28by%20ref%29))
  (if (Actor|ActorHasTag OtherActor "PB")
    (Variables|Default|Setmultiplier 1.2)
    (CallFunction|ApplyReward)))

(event OnComponentBeginOverlap(Reward1.2_2)
  (params (OverlappedComponent :type Primitive%20Component%20Object%20Reference) (OtherActor :type Actor%20Object%20Reference) (OtherComp :type Primitive%20Component%20Object%20Reference) (OtherBodyIndex :type Integer) (bFromSweep :type Boolean) (SweepResult :type Hit%20Result%20Structure%20%28by%20ref%29))
  (if (Actor|ActorHasTag OtherActor "PB")
    (Variables|Default|Setmultiplier 1.2)
    (CallFunction|ApplyReward)))

(event OnComponentBeginOverlap(Reward2_2)
  (params (OverlappedComponent :type Primitive%20Component%20Object%20Reference) (OtherActor :type Actor%20Object%20Reference) (OtherComp :type Primitive%20Component%20Object%20Reference) (OtherBodyIndex :type Integer) (bFromSweep :type Boolean) (SweepResult :type Hit%20Result%20Structure%20%28by%20ref%29))
  (if (Actor|ActorHasTag OtherActor "PB")
    (Variables|Default|Setmultiplier 2.0)
    (CallFunction|ApplyReward)))

(event OnComponentBeginOverlap(Reward_2_1)
  (params (OverlappedComponent :type Primitive%20Component%20Object%20Reference) (OtherActor :type Actor%20Object%20Reference) (OtherComp :type Primitive%20Component%20Object%20Reference) (OtherBodyIndex :type Integer) (bFromSweep :type Boolean) (SweepResult :type Hit%20Result%20Structure%20%28by%20ref%29))
  (if (Actor|ActorHasTag OtherActor "PB")
    (Variables|Default|Setmultiplier 2.0)
    (CallFunction|ApplyReward)))

(event OnComponentBeginOverlap(Reward_2.5_1)
  (params (OverlappedComponent :type Primitive%20Component%20Object%20Reference) (OtherActor :type Actor%20Object%20Reference) (OtherComp :type Primitive%20Component%20Object%20Reference) (OtherBodyIndex :type Integer) (bFromSweep :type Boolean) (SweepResult :type Hit%20Result%20Structure%20%28by%20ref%29))
  (if (Actor|ActorHasTag OtherActor "PB")
    (Variables|Default|Setmultiplier 2.2)
    (CallFunction|ApplyReward)))

(event OnComponentBeginOverlap(Reward2.5_2)
  (params (OverlappedComponent :type Primitive%20Component%20Object%20Reference) (OtherActor :type Actor%20Object%20Reference) (OtherComp :type Primitive%20Component%20Object%20Reference) (OtherBodyIndex :type Integer) (bFromSweep :type Boolean) (SweepResult :type Hit%20Result%20Structure%20%28by%20ref%29))
  (if (Actor|ActorHasTag OtherActor "PB")
    (Variables|Default|Setmultiplier 2.2)
    (CallFunction|ApplyReward)))

(event Custom|ApplyReward
  (bind _output_get (Variables|Default|Setstats (.OutItem (Utilities|Array|Random (Variables|Default|GetgambledStats)))))
  (bind _value (Default|GetStats (stale EventUseMachine playerRef) _output_get))
  (Default|AddStats (stale EventUseMachine playerRef) _output_get (/ (* _value (Variables|Default|Getmultiplier)) 1e+02))
  (|CallParentFunction 0))

(event Custom|SpawnBall
  (bind _ballspawnlimit1 (Variables|Default|GetBallSpawnLimit1))
  (bind _relativelocation (Variables|/Script/Engine.SceneComponent|GetRelativeLocation _ballspawnlimit1))
  (bind (_x _y _z) (Math|Vector|BreakVector _relativelocation))
  (Game|SpawnActorfromClass "/Game/GAME_Casino/Folder_Adrien/BP_PlinkoBall.BP_PlinkoBall_C" (Math|Conversions|ToTransform(Vector) (Math|Transform|TransformLocation (Transformation|GetActorTransform) (Math|Vector|MakeVector _x (Math|Random|RandomFloatinRange _y (.Y (Math|Vector|BreakVector (Variables|/Script/Engine.SceneComponent|GetRelativeLocation (Variables|Default|GetBallSpawnLimit2))))) _z))) "Undefined" "MultiplyWithRoot" 0 0))

(event EventBeginPlay
  (|CallParentFunction) ; This node is disabled and will not be called.\nDrag off pins to build functionality.
)

(event EventUseMachine
  (params (playerRef :type BP%20First%20Person%20Character%20Object%20Reference))
  (CallFunction|SpawnBall))

(fn ConstructionScript
  (|CallParentFunction))