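; Casino dice machine that gambles a random stat of the player on the total of several thrown dice.
; On use, it spawns four dice stacked above a platform, which two timelines lower and then raise before throwing them.
; Dice report back through AddResult while the machine polls until all results arrive.
; It converts the sum's deviation from an average into a percentage and passes it with the stat to the parent machine logic.
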(event Custom|TriggerThrow
  (bind _plateforme (Variables|Default|GetPlateforme))
  (bind _relativelocation (Variables|/Script/Engine.SceneComponent|GetRelativeLocation _plateforme))
  (bind (_x _y _z) (Math|Vector|BreakVector _relativelocation))
  (bind _firsttrigger (Timeline|Timeline PlayFromStart)
    (:Update
      (Transformation|SetRelativeLocation _plateforme (Math|Vector|MakeVector _x _y (Math|Float|Lerp _z (- _z 2.0) _firsttrigger)) false false))
    (:Finished
      (Utilities|FlowControl|Delay 1.0)
      (CallFunction|ThrowAll))))

(event Custom|ThrowAll
  (bind _plateforme (Variables|Default|GetPlateforme))
  (bind _relativelocation (Variables|/Script/Engine.SceneComponent|GetRelativeLocation _plateforme))
  (bind (_x _y _z) (Math|Vector|BreakVector _relativelocation))
  (bind _alpha (Timeline|Timeline_0 PlayFromStart)
    (:Update
      (Transformation|SetRelativeLocation _plateforme (Math|Vector|MakeVector _x _y (Math|Float|Lerp _z (+ _z 15.0) _alpha)) false false))
    (:Finished
      (for _array_element (Variables|Default|GetDice)
        (Default|ThrowDice _array_element))
      (CallFunction|WaitforAllResult))))

(event Custom|WaitForAllResult
  (if (== (Utilities|Array|Length (Variables|Default|Getresultarray)) (Utilities|Array|Length (Variables|Default|GetDice))) :!label _label
    (for _array_element (Variables|Default|Getresultarray)
      (Variables|Default|SetfullResult (+ _array_element (Variables|Default|GetfullResult))))
    (bind _output_get (Variables|Default|Setstats (.OutItem (Utilities|Array|Random (Variables|Default|GetgambledStats)))))
    (|CallParentFunction (Variables|Default|GetplayerRef) (* (/ (- (Variables|Default|GetfullResult) (Variables|Default|Getmoyenne)) (- 24.0 14.0)) 5.0) _output_get false)
    (else
      (Utilities|FlowControl|Delay 0.5)
      (goto _label))))

(event Custom|AddResult
  (params (result :type Integer))
  (Utilities|Array|Add (Variables|Default|Getresultarray) result))

(event EventUseMachine
  (params (playerRef :type BP%20First%20Person%20Character%20Object%20Reference) (addedPercent :type Float%20%28double-precision%29) (stats :type E_Stats%20Enum :default "NewEnumerator0") (notEnded :type Boolean))
  (Variables|Default|SetplayerRef playerRef)
  (Utilities|Array|Clear (Variables|Default|GetDice))
  (Utilities|Array|Clear (Variables|Default|Getresultarray))
  (Variables|Default|SetfullResult 0.0)
  (for _index (range 0 3)
    (bind _returnvalue (Game|SpawnActorfromClass "/Game/GAME_Casino/Folder_Adrien/BP_ThrowableDice.BP_ThrowableDice_C" (Math|Conversions|ToTransform(Vector) (+ (Transformation|GetWorldLocation (Variables|Default|GetPlateforme)) (Math|Vector|MakeVector 0.0 0.0 (* _index 5e+01)))) "Undefined" "MultiplyWithRoot" 0 0))
    (Default|SetMachine _returnvalue self)
    (Utilities|Array|Add (Variables|Default|GetDice) _returnvalue)
    (Utilities|FlowControl|Delay 0.2)
    (CallFunction|TriggerThrow)))

(fn ConstructionScript
  (|CallParentFunction))