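; BP_MachineGoldDigger is a casino machine that runs a short timed minigame, played by either screaming or clicking, chosen randomly at BeginPlay.
; On use it shows a WB_GoldDigger widget, then after a countdown delay enables Tick to poll the player's voice level or input to count left clicks.
; After a five-second window, it awards the score times a random multiplier to a player stat, removes the widget and destroys itself.
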(event Input|EnhancedActionEvents|EnhancedInputActionIA_LeftClick
  (params (ActionValue :type Boolean) (ElapsedSeconds :type Float%20%28double-precision%29) (TriggeredSeconds :type Float%20%28double-precision%29) (InputAction :type Input%20Action%20Object%20Reference :default "/Game/Input/Actions/IA_LeftClick.IA_LeftClick"))
  (:Started
    (Audio|PlaySound2D "/Game/GAME_Casino/Folder_Adrien/ImportSon/Click/Click_Cue.Click_Cue" 1.0 1.0 0.0 0 0)
    (Math|Float|IncrementFloat (Variables|Default|GettotalScore)
      (:%20%20
        (Default|AddScore (Variables|Default|GetcurrentWidget) 1.0)))))

(event EventTick
  (params (DeltaSeconds :type Float%20%28single-precision%29))
  (if (and (and (Variables|Default|Getstart) (Variables|Default|GetisScream)) (> (Variables|/Game/FirstPerson/Blueprints/BP_FirstPersonCharacter.BP_FirstPersonCharacter_C|GetvoiceValue (stale EventUseMachine playerRef)) 0.5))
    (Variables|Default|SettotalScore (+ (Variables|Default|GettotalScore) 0.5))
    (Default|AddScore (Variables|Default|GetcurrentWidget) (+ (Variables|Default|GettotalScore) 0.5))))

(event EventBeginPlay
  (Variables|Default|SetisScream (Math|Random|RandomBool))
  (|CallParentFunction))

(event EventUseMachine
  (params (playerRef :type BP%20First%20Person%20Character%20Object%20Reference) (addedPercent :type Float%20%28double-precision%29) (stats :type E_Stats%20Enum :default "NewEnumerator0") (notEnded :type Boolean))
  (bind _returnvalue (UserInterface|CreateWidget "/Game/GAME_Casino/Folder_Adrien/WB_GoldDigger.WB_GoldDigger_C"))
  (UserInterface|Viewport|AddtoViewport _returnvalue 0)
  (bind _output_get (Variables|Default|SetcurrentWidget _returnvalue))
  (Default|SetInfo _returnvalue (Variables|Default|GetisScream) self)
  (Utilities|FlowControl|Delay 3.0)
  (if (Variables|Default|GetisScream)
    (Actor|Tick|SetActorTickEnabled true)
    (else
      (Input|EnableInput (Game|GetPlayerController 0))))
  (Variables|Default|SettotalScore 0.0)
  (Variables|Default|Setstart true)
  ;[0.15 0.15 0.15 0.5] Click
  (Utilities|FlowControl|Delay 5.0)
  (Default|AddStats playerRef "NewEnumerator1" (* (Variables|Default|GettotalScore) (Math|Random|RandomFloatinRange 1.0 4.0)))
  (Widget|RemovefromParent (Variables|Default|GetcurrentWidget))
  (Actor|DestroyActor))

(fn ConstructionScript
  (|CallParentFunction))