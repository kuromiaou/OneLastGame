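; Throwable casino die that randomizes its orientation when thrown, then reports the face it lands on to its assigned machine.
; On the server, BeginPlay collects the Arrow components under the die, one marking each face.
; After a delay, it finds the arrow pointing roughly world-up and sends the last digit of its name as the result.
; It retries until a face qualifies, then destroys itself after a pause.
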(event Custom|ThrowDice
  (bind _returnvalue (Math|Random|RandomFloatinRange 0.0 3.6e+02))
  (Transformation|SetWorldRotation (Variables|Default|GetDice) (Math|Rotator|MakeRotator _returnvalue _returnvalue _returnvalue) false false)
  (Utilities|FlowControl|Delay 5.0)
  (CallFunction|Result))

(event Custom|Result
  (bind _array_element (Utilities|Array|ForEachLoopwithBreak (Variables|Default|GetarrowArray) :!label _label)
    (:LoopBody
      (if (Utilities|Operators|EqualEqual (Math|Vector|GetForwardVector _array_element) "0.000000,0.000000,1.000000" 0.5)
        (Variables|Default|Setfound? (Utilities|Operators|EqualEqual (Math|Vector|GetForwardVector _array_element) "0.000000,0.000000,1.000000" 0.5))
        (Default|AddResult (Variables|Default|GetcurrentMachine) (Math|Conversions|ToInteger(Byte) (Utilities|Array|Get(acopy) (Utilities|String|GetCharacterArrayfromString (Utilities|GetObjectName _array_element)) (Utilities|Array|LastIndex (Utilities|String|GetCharacterArrayfromString (Utilities|GetObjectName _array_element))))))
        (goto _label Break)))
    (:Completed
      (if (Variables|Default|Getfound?)
        (Utilities|FlowControl|Delay 5.0)
        (Actor|DestroyActor)
        (else
          (Utilities|FlowControl|Delay 0.2)
          (goto _label))))))

(event Custom|SetMachine
  (params (machine :type BP%20Machine%20Dé%20Object%20Reference))
  (Variables|Default|SetcurrentMachine machine))

(event EventBeginPlay
  (Networking|SwitchHasAuthority
    (:Authority
      (for _array_element (Components|GetChildrenComponents (Variables|Default|GetDice) false)
        (bind _asarrow_component (Utilities|Casting|CastToArrowComponent _array_element))
        (Utilities|Array|Add (Variables|Default|GetarrowArray) _asarrow_component)))))

(fn ConstructionScript)