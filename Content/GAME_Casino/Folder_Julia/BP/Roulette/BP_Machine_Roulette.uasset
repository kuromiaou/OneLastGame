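; Casino roulette machine that gambles one of the player's stats when used.
; UseMachine plays a timeline that spins the GizRoulette component by adding world yaw on each update.
; When the spin finishes, it calls the parent UseMachine with the player, a random stat from GambledStats and a random percentage change that can be a loss or a gain.
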(event EventBeginPlay
  (|CallParentFunction) ; This node is disabled and will not be called.\nDrag off pins to build functionality.
)

(event Collision|EventActorBeginOverlap
  (params (OtherActor :type Actor%20Object%20Reference)))

(event EventTick
  (params (DeltaSeconds :type Float%20%28single-precision%29)))

(event EventUseMachine
  (params (playerRef :type BP%20First%20Person%20Character%20Object%20Reference) (addedPercent :type Float%20%28double-precision%29) (stats :type E_Stats%20Enum :default "NewEnumerator0") (notEnded :type Boolean))
  (bind _rotation (Timeline|Timeline PlayFromStart)
    (:Update
      (Transformation|AddWorldRotation (Variables|Default|GetGizRoulette) (Math|Rotator|MakeRotator 0.0 0.0 _rotation) false false))
    (:Finished
      (|CallParentFunction playerRef (Math|Random|RandomFloatinRange -1e+01 25.0) (.OutItem (Utilities|Array|Random (Variables|Default|GetgambledStats))) false))))

(fn ConstructionScript
  (|CallParentFunction))