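; Casino weapon box machine that displays a copy of the player's current weapon and randomly alters its stats.
; UseMachine plays a timeline that, on every update, spawns a weapon copy at WeaponPos, yaws it by a speed curve and shifts each stat by -5% to +20%, compounding.
; On finish it calls the parent UseMachine and destroys the last spawned copy.
; Tourniquet is a stub that applies zero rotation.
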(event EventTick
  (params (DeltaSeconds :type Float%20%28single-precision%29)))

(event EventUseMachine
  (params (playerRef :type BP%20First%20Person%20Character%20Object%20Reference) (addedPercent :type Float%20%28double-precision%29) (stats :type E_Stats%20Enum :default "NewEnumerator0") (notEnded :type Boolean))
  (bind _currentweapon (Variables|/Game/FirstPerson/Blueprints/BP_FirstPersonCharacter.BP_FirstPersonCharacter_C|GetCurrentWeapon playerRef))
  (bind _enum_weapons_current_stats (Variables|/Game/GAME_Shooter/Folder_Maxime/FOLDER_GENERAL_WEAPON_CLASS/BP_MOTHER_WEAPON_CLASS.BP_MOTHER_WEAPON_CLASS_C|GetENUM_Weapons_Current_Stats _currentweapon))
  (bind _speedcurve (Timeline|Timeline PlayFromStart)
    (:Update
      (bind _weaponref (CallFunction|CreateRefRotation _currentweapon))
      (Transformation|AddActorLocalRotation _weaponref (Math|Rotator|MakeRotator 0.0 0.0 (* (stale EventTick DeltaSeconds) _speedcurve)) false false)
      (for _index (range 0 (Utilities|Map|GetLastIndex _enum_weapons_current_stats))
        (Utilities|Map|Add _enum_weapons_current_stats (.Key (Utilities|Map|GetKeyValueByIndex _enum_weapons_current_stats _index)) (+ (.Value (Utilities|Map|GetKeyValueByIndex _enum_weapons_current_stats _index)) (* (.Value (Utilities|Map|GetKeyValueByIndex _enum_weapons_current_stats _index)) (/ (Math|Random|RandomFloatinRange -5.0 2e+01) 1e+02))))))
    (:Finished
      (|CallParentFunction playerRef 0.0 "NewEnumerator0" false)
      (Actor|DestroyActor _weaponref))))

(fn ConstructionScript
  (|CallParentFunction))

(fn Tourniquet
  (if (not (> (Variables|Default|Gettimer) 3.14))
    (Transformation|AddActorLocalRotation "0, 0, 0" false false)))

(fn CreateRefRotation
  (params (weapon :type BP%20MOTHER%20WEAPON%20CLASS%20Object%20Reference))
  (bind _returnvalue (Game|SpawnActorfromClass (Utilities|GetClass weapon) (Math|Transform|MakeTransform (Transformation|GetWorldLocation (Variables|Default|GetWeaponPos)) "0, 0, 0" "1.000000,1.000000,1.000000") "Undefined" "MultiplyWithRoot" 0 0))
  (return _returnvalue))