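; Permanent passive "Ammo" for the casino game, meant to give a 34% chance to refund ammo spent when shooting.
; ApplyEffects reads one stat from the passed Passif and, on a random roll, calls AddStats on a different stat with that value plus one.
; Its guard compares the read stat to itself minus one, so it does not actually detect a shot.
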(event EventApplyEffects
  (params (Passif :type BP%20First%20Person%20Character%20Child%20Object%20Reference))
  ;[0 0 0 0.5] Ammo : when you shoot with your weapon, you have 34% chance to get back your shooted ammo
  (bind _value (Default|GetStats Passif "NewEnumerator9"))
  (if (!= _value (- _value 1.0))
    (if (<= (Math|Random|RandomFloat) 0.34)
      (Default|AddStats Passif "NewEnumerator8" (+ _value 1.0)))))

(fn ConstructionScript
  (|CallParentFunction))