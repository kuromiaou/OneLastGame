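; Permanent passive "Adrenaline" for the casino game, meant to boost the player's stats when a monitored stat is low.
; ApplyEffects reads stats from BP_FirstPersonCharacter and, below a threshold, adds multiples of two stats' current values back onto them via AddStats.
; As written, the threshold evaluates to zero, and a second stat read goes unused.
; The boost is never reverted here, and the parent ApplyEffects is not called.
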(event EventApplyEffects
  (params (Passif :type BP%20First%20Person%20Character%20Child%20Object%20Reference))
  (bind _asbp_first_person_character (Utilities|Casting|CastToBP_FirstPersonCharacter (Game|GetPlayerCharacter 0)))
  (bind _value (Default|GetStats _asbp_first_person_character "NewEnumerator0"))
  (Default|GetStats _asbp_first_person_character "NewEnumerator18")
  (if (<= _value (* 0.0 0.8))
    (bind _value_2 (Default|GetStats _asbp_first_person_character "NewEnumerator2"))
    (Default|AddStats _asbp_first_person_character "NewEnumerator2" (* _value_2 1.1))
    (bind _value_3 (Default|GetStats _asbp_first_person_character "NewEnumerator1"))
    (Default|AddStats _asbp_first_person_character "NewEnumerator1" (* _value_3 1.2))))

(fn ConstructionScript
  (|CallParentFunction))