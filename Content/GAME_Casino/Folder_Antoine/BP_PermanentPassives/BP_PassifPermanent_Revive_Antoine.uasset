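; Permanent passive Blueprint meant to revive the owner at zero health with full health and three seconds of invincibility.
; ApplyEffects clears its invincibility flag, reads two stats from the Passif input, apparently max and current health.
; When current health is zero or below, it sets the flag and adds the max value to health.
; The invincibility branch is empty, with no timer or protection implemented here.
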(event EventApplyEffects
  (params (Passif :type BP%20First%20Person%20Character%20Child%20Object%20Reference))
  ;[0.15 0.1077 0.007854 0.5] Revive : when you reach 0% of your health, you recover 100% of your health and are invicible for 3 secondes
  (Variables|Default|SetBP_PassifPerma_Invicible false)
  (bind _value (Default|GetStats Passif "NewEnumerator18"))
  (bind _value_2 (Default|GetStats Passif "NewEnumerator0"))
  (if (<= _value_2 0.0)
    (Variables|Default|SetBP_PassifPerma_Invicible true)
    (Default|AddStats Passif "NewEnumerator0" _value)
    (if (Variables|Default|GetBP_PassifPerma_Invicible)
      _)))

(fn ConstructionScript
  (|CallParentFunction))