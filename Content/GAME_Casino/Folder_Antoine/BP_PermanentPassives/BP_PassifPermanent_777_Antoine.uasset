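; Permanent passive "777" for the casino game, apparently unfinished.
; ApplyEffects reads several stats from the first-person player, stores two in ValueStats, then starts a looping timer that fires Passif777.
; Passif777 rolls a random boolean but neither outcome does anything, and the stored stats are never used.
; Other nodes that would add more stats to ValueStats are disconnected.
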(event Custom|Passif%20777
  (if (Math|Random|RandomBool)
    _))

(event EventApplyEffects
  (params (Passif :type BP%20First%20Person%20Character%20Child%20Object%20Reference))
  (bind _bp_firstperson (Variables|Default|Getbp_firstperson))
  (bind _value (Default|GetStats _bp_firstperson "NewEnumerator2"))
  (bind _value_2 (Default|GetStats _bp_firstperson "NewEnumerator18"))
  (Default|GetStats _bp_firstperson "NewEnumerator4")
  (bind _value_3 (Default|GetStats _bp_firstperson "NewEnumerator6"))
  (bind _value_4 (Default|GetStats _bp_firstperson "NewEnumerator7"))
  (Default|GetStats _bp_firstperson "NewEnumerator10")
  (bind _value_5 (Default|GetStats _bp_firstperson "NewEnumerator11"))
  (Utilities|Array|Add (Variables|Default|GetvalueStats) _value_5)
  (bind _value_6 (Default|GetStats _bp_firstperson "NewEnumerator17"))
  (Utilities|Array|Add (Variables|Default|GetvalueStats) _value_6)
  (Utilities|Time|SetTimerbyEvent (delegate Custom|Passif%20777) 15.0 true))

(fn ConstructionScript
  (|CallParentFunction))