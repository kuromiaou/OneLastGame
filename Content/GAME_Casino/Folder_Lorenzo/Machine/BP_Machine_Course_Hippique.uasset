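; Casino horse-race betting machine: the player bets on one of four colored horses to gain or lose a random gambled stat.
; UseMachine line-traces from the player camera to a color button, starts the race, then polls until it finishes.
; Tick rerolls speeds and moves horses with random delays until one collider overlaps the finish.
; EndRace ranks horses by distance to the line, and the picked horse's rank sets the percent passed to the parent.
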(event Custom|OnComponentBeginOverlap_Event
  (params (OverlappedComponent :type Primitive%20Component%20Object%20Reference) (OtherActor :type Actor%20Object%20Reference) (OtherComp :type Primitive%20Component%20Object%20Reference) (OtherBodyIndex :type Integer) (bFromSweep :type Boolean) (SweepResult :type Hit%20Result%20Structure%20%28by%20ref%29))
  (Collision|AssignOnComponentBeginOverlap OverlappedComponent (delegate Custom|OnComponentBeginOverlap_Event)))

(event EventBeginPlay
  (|CallParentFunction))

(event Collision|EventActorBeginOverlap
  (params (OtherActor :type Actor%20Object%20Reference)))

(event EventTick
  (params (DeltaSeconds :type Float%20%28single-precision%29))
  (bind (_yellow_horse _x _returnvalue _z _green_horse _x2 _returnvalue2 _z2 _red_horse _x3 _returnvalue3 _z3 _blue_horse _x4 _returnvalue4 _z4) (|CalculSpeed))
  (Utilities|FlowControl|Sequence
    (:then_0
      (CallFunction|EndRace))
    (:then_1
      (|SpeedRandom))
    (:then_2
      (if (Variables|Default|GetRaceStarted)
        (if (not (Variables|Default|GetRaceFinished))
          (Utilities|FlowControl|Sequence
            (:then_0
              (|DelayRace :!label _label
                (:then
                  (Transformation|SetRelativeLocation _yellow_horse (Math|Vector|MakeVector _x _returnvalue _z) false false))
                (:then2
                  (Transformation|SetRelativeLocation _green_horse (Math|Vector|MakeVector _x2 _returnvalue2 _z2) false false))
                (:then3
                  (Transformation|SetRelativeLocation _red_horse (Math|Vector|MakeVector _x3 _returnvalue3 _z3) false false))
                (:then4
                  (Transformation|SetRelativeLocation _blue_horse (Math|Vector|MakeVector _x4 _returnvalue4 _z4) false false))))
            (:then_1
              (goto _label execute2))
            (:then_2
              (goto _label execute3))
            (:then_3
              (goto _label execute4))))))))

(event EventUseMachine
  (params (playerRef :type BP%20First%20Person%20Character%20Object%20Reference) (addedPercent :type Float%20%28double-precision%29) (stats :type E_Stats%20Enum :default "NewEnumerator0") (notEnded :type Boolean))
  (bind _gambledstats (Variables|Default|GetgambledStats))
  (bind _outitem (Utilities|Array|Random _gambledstats))
  (bind _output_get (Variables|Default|SetPlayer%20ref playerRef))
  (|CallParentFunction _output_get 0.0 "NewEnumerator0" true)
  (bind _outhit (Collision|LineTraceByChannel (Transformation|GetWorldLocation (Variables|/Game/FirstPerson/Blueprints/BP_FirstPersonCharacter.BP_FirstPersonCharacter_C|GetFirstPersonCamera (Variables|Default|GetPlayer%20ref))) (+ (Transformation|GetWorldLocation (Variables|/Game/FirstPerson/Blueprints/BP_FirstPersonCharacter.BP_FirstPersonCharacter_C|GetFirstPersonCamera (Variables|Default|GetPlayer%20ref))) (* (Math|Vector|GetForwardVector (Variables|/Game/FirstPerson/Blueprints/BP_FirstPersonCharacter.BP_FirstPersonCharacter_C|GetFirstPersonCamera (Variables|Default|GetPlayer%20ref))) 4e+02)) "TraceTypeQuery1" false (Utilities|Array|MakeArray (Variables|Default|GetPlayer%20ref)) "ForDuration" false "(R=0.217092,G=0.000000,B=1.000000,A=1.000000)" "(R=0.000000,G=1.000000,B=0.744368,A=1.000000)" 1e+01))
  (Utilities|FlowControl|Sequence
    (:then_0
      (if (.ReturnValue (|CheckHit (.hitactor _outhit) (.hitcomponent _outhit) (.hitcomponent _outhit) (.hitcomponent _outhit) (.hitcomponent _outhit)))
        (Variables|Default|SetColorChoosed "NewEnumerator0")
        (Variables|Default|SetRaceStarted true :!label _label)
        (if (Variables|Default|GetRaceFinished) :!label _label_2
          (for (_array_element _array_index) (Variables|Default|GetNewArray)
            (if (Utilities|Enum|Equal(Enum) (.horse _array_element) (Variables|Default|GetColorChoosed))
              (switch int _array_index
                (:0
                  (|CallParentFunction (Variables|Default|GetPlayer%20ref) (Math|Random|RandomFloatinRange -5.0 -3.0) _outitem false))
                (:1
                  (|CallParentFunction (Variables|Default|GetPlayer%20ref) (Math|Random|RandomFloatinRange -2.0 -1.0) _outitem false))
                (:2
                  (|CallParentFunction (Variables|Default|GetPlayer%20ref) (Math|Random|RandomFloatinRange 2.0 3.0) _outitem false))
                (:3
                  (|CallParentFunction (Variables|Default|GetPlayer%20ref) (Math|Random|RandomFloatinRange 4.0 6.0) _outitem false)))))
          (else
            (Utilities|FlowControl|Delay 0.5)
            (goto _label_2)))))
    (:then_1
      (if (.ReturnValue2 (|CheckHit (.hitactor _outhit) (.hitcomponent _outhit) (.hitcomponent _outhit) (.hitcomponent _outhit) (.hitcomponent _outhit)))
        (Variables|Default|SetColorChoosed "NewEnumerator3")
        (goto _label)))
    (:then_2
      (if (.ReturnValue3 (|CheckHit (.hitactor _outhit) (.hitcomponent _outhit) (.hitcomponent _outhit) (.hitcomponent _outhit) (.hitcomponent _outhit)))
        (Variables|Default|SetColorChoosed "NewEnumerator2")
        (goto _label)))
    (:then_3
      (if (.ReturnValue4 (|CheckHit (.hitactor _outhit) (.hitcomponent _outhit) (.hitcomponent _outhit) (.hitcomponent _outhit) (.hitcomponent _outhit)))
        (Variables|Default|SetColorChoosed "NewEnumerator1")
        (goto _label)))
    (:then_4
      (if (.ReturnValue5 (|CheckHit (.hitactor _outhit) (.hitcomponent _outhit) (.hitcomponent _outhit) (.hitcomponent _outhit) (.hitcomponent _outhit)))
        (Development|PrintString "Clic sur un bouton couillon !!")))))

(fn ConstructionScript
  (|CallParentFunction))

(fn EndRace
  (if (not (Variables|Default|GetRaceFinished))
    (Utilities|FlowControl|Sequence
      (:then_0
        (if (Class|PrimitiveComponent|IsOverlappingComponent (Variables|Default|GetBlueHorseCollider) (Variables|Default|GetEndCollider))
          (Development|PrintString "Blue win")
          (Variables|Default|SetWinnerColor "NewEnumerator1")
          (Variables|Default|SetRaceFinished false :!label _label)
          (Utilities|FlowControl|Sequence
            (:then_0
              (Utilities|Array|Add (Variables|Default|GetRaceEntry) (Utilities|Struct|MakeS_RaceEntry "NewEnumerator1" (Math|Vector|Distance(Vector) (Math|Vector|MakeVector 0.0 (.y (Transformation|GetWorldLocation (Variables|Default|GetBlueHorseCollider))) 0.0) (Math|Vector|MakeVector 0.0 (.y (Transformation|GetWorldLocation (Variables|Default|GetEndCollider))) 0.0)))))
            (:then_1
              (Utilities|Array|Add (Variables|Default|GetRaceEntry) (Utilities|Struct|MakeS_RaceEntry "NewEnumerator0" (Math|Vector|Distance(Vector) (Math|Vector|MakeVector 0.0 (.y (Transformation|GetWorldLocation (Variables|Default|GetRedHorseCollider))) 0.0) (Math|Vector|MakeVector 0.0 (.y (Transformation|GetWorldLocation (Variables|Default|GetEndCollider))) 0.0)))))
            (:then_2
              (Utilities|Array|Add (Variables|Default|GetRaceEntry) (Utilities|Struct|MakeS_RaceEntry "NewEnumerator3" (Math|Vector|Distance(Vector) (Math|Vector|MakeVector 0.0 (.y (Transformation|GetWorldLocation (Variables|Default|GetGreenHorseCollider))) 0.0) (Math|Vector|MakeVector 0.0 (.y (Transformation|GetWorldLocation (Variables|Default|GetEndCollider))) 0.0)))))
            (:then_3
              (Utilities|Array|Add (Variables|Default|GetRaceEntry) (Utilities|Struct|MakeS_RaceEntry "NewEnumerator2" (Math|Vector|Distance(Vector) (Math|Vector|MakeVector 0.0 (.y (Transformation|GetWorldLocation (Variables|Default|GetYellowHorseCollider))) 0.0) (Math|Vector|MakeVector 0.0 (.y (Transformation|GetWorldLocation (Variables|Default|GetEndCollider))) 0.0)))))
            (:then_4
              (CallFunction|Sort)
              (for _array_element (Variables|Default|GetNewArray)
                (Development|PrintString (Utilities|String|EnumtoString (.horse _array_element))))
              (Variables|Default|SetRaceFinished true)))))
      (:then_1
        (if (Class|PrimitiveComponent|IsOverlappingComponent (Variables|Default|GetRedHorseCollider) (Variables|Default|GetEndCollider))
          (Development|PrintString "red win")
          (Variables|Default|SetWinnerColor "NewEnumerator0")
          (goto _label)))
      (:then_2
        (if (Class|PrimitiveComponent|IsOverlappingComponent (Variables|Default|GetGreenHorseCollider) (Variables|Default|GetEndCollider))
          (Development|PrintString "Green win")
          (Variables|Default|SetWinnerColor "NewEnumerator3")
          (goto _label)))
      (:then_3
        (if (Class|PrimitiveComponent|IsOverlappingComponent (Variables|Default|GetYellowHorseCollider) (Variables|Default|GetEndCollider))
          (Development|PrintString "Yellow win")
          (Variables|Default|SetWinnerColor "NewEnumerator2")
          (goto _label))))))

(fn Sort
  (bind _raceentry (Variables|Default|GetRaceEntry))
  (for (_array_element _array_index) _raceentry :!label _label
    (if (== _array_index 0)
      (LocalVariables|SetlastDistance (.Distance (Utilities|Struct|BreakS_RaceEntry _array_element)))
      (elif (not (> (LocalVariables|GetlastDistance) (.Distance (Utilities|Struct|BreakS_RaceEntry _array_element))))
        (LocalVariables|SetlastDistance (.Distance (Utilities|Struct|BreakS_RaceEntry _array_element))))))
  (for (_array_element_2 _array_index_2) _raceentry
    (if (== (.Distance (Utilities|Struct|BreakS_RaceEntry _array_element_2)) (LocalVariables|GetlastDistance))
      (Utilities|Array|Add (Variables|Default|GetNewArray) _array_element_2)
      (Utilities|Array|RemoveIndex (Variables|Default|GetRaceEntry) _array_index_2)))
  (bind _result (Math|Integer|IncrementInt (LocalVariables|GettotalLoop))
    (:%20%20
      (if (>= _result 4)
        (return)
        (else
          (goto _label))))))