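; BP_EmptyRoom4 is a room variant in the casino's procedural generation set that fills itself with box props at startup.
; After the parent BeginPlay, it spawns BP_box_bois actors at its Box marker components, each with a random yaw.
; Box4 receives two spawns, and the Box2, Box3 and first Box4 spawns use a zero Z scale, unlike the others.
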(event EventBeginPlay
  (|CallParentFunction)
  (Game|SpawnActorfromClass "/Game/GAME_Shooter/Folder_Charly/Chaos/PropsChaos/BP_box_bois.BP_box_bois_C" (Math|Transform|MakeTransform (Transformation|GetWorldLocation (Variables|Default|GetBox1)) (Math|Rotator|MakeRotator 0.0 0.0 (Math|Random|RandomFloatinRange 0.0 3.6e+02)) "1.000000,1.000000,1.000000") "Undefined" "MultiplyWithRoot" 0 0)
  (Game|SpawnActorfromClass "/Game/GAME_Shooter/Folder_Charly/Chaos/PropsChaos/BP_box_bois.BP_box_bois_C" (Math|Transform|MakeTransform (Transformation|GetWorldLocation (Variables|Default|GetBox2)) (Math|Rotator|MakeRotator 0.0 0.0 (Math|Random|RandomFloatinRange 0.0 3.6e+02)) "1.0,1.0,0.0") "Undefined" "MultiplyWithRoot" 0 0)
  (Game|SpawnActorfromClass "/Game/GAME_Shooter/Folder_Charly/Chaos/PropsChaos/BP_box_bois.BP_box_bois_C" (Math|Transform|MakeTransform (Transformation|GetWorldLocation (Variables|Default|GetBox3)) (Math|Rotator|MakeRotator 0.0 0.0 (Math|Random|RandomFloatinRange 0.0 3.6e+02)) "1.0,1.0,0.0") "Undefined" "MultiplyWithRoot" 0 0)
  (Game|SpawnActorfromClass "/Game/GAME_Shooter/Folder_Charly/Chaos/PropsChaos/BP_box_bois.BP_box_bois_C" (Math|Transform|MakeTransform (Transformation|GetWorldLocation (Variables|Default|GetBox4)) (Math|Rotator|MakeRotator 0.0 0.0 (Math|Random|RandomFloatinRange 0.0 3.6e+02)) "1.0,1.0,0.0") "Undefined" "MultiplyWithRoot" 0 0)
  (Game|SpawnActorfromClass "/Game/GAME_Shooter/Folder_Charly/Chaos/PropsChaos/BP_box_bois.BP_box_bois_C" (Math|Transform|MakeTransform (Transformation|GetWorldLocation (Variables|Default|GetBox4)) (Math|Rotator|MakeRotator 0.0 0.0 (Math|Random|RandomFloatinRange 0.0 3.6e+02)) "1.000000,1.000000,1.000000") "Undefined" "MultiplyWithRoot" 0 0)
  (Game|SpawnActorfromClass "/Game/GAME_Shooter/Folder_Charly/Chaos/PropsChaos/BP_box_bois.BP_box_bois_C" (Math|Transform|MakeTransform (Transformation|GetWorldLocation (Variables|Default|GetBox5)) (Math|Rotator|MakeRotator 0.0 0.0 (Math|Random|RandomFloatinRange 0.0 3.6e+02)) "1.000000,1.000000,1.000000") "Undefined" "MultiplyWithRoot" 0 0)
  (Game|SpawnActorfromClass "/Game/GAME_Shooter/Folder_Charly/Chaos/PropsChaos/BP_box_bois.BP_box_bois_C" (Math|Transform|MakeTransform (Transformation|GetWorldLocation (Variables|Default|GetBox6)) (Math|Rotator|MakeRotator 0.0 0.0 (Math|Random|RandomFloatinRange 0.0 3.6e+02)) "1.000000,1.000000,1.000000") "Undefined" "MultiplyWithRoot" 0 0)
  (Game|SpawnActorfromClass "/Game/GAME_Shooter/Folder_Charly/Chaos/PropsChaos/BP_box_bois.BP_box_bois_C" (Math|Transform|MakeTransform (Transformation|GetWorldLocation (Variables|Default|GetBox7)) (Math|Rotator|MakeRotator 0.0 0.0 (Math|Random|RandomFloatinRange 0.0 3.6e+02)) "1.000000,1.000000,1.000000") "Undefined" "MultiplyWithRoot" 0 0)
  (Game|SpawnActorfromClass "/Game/GAME_Shooter/Folder_Charly/Chaos/PropsChaos/BP_box_bois.BP_box_bois_C" (Math|Transform|MakeTransform (Transformation|GetWorldLocation (Variables|Default|GetBox8)) (Math|Rotator|MakeRotator 0.0 0.0 (Math|Random|RandomFloatinRange 0.0 3.6e+02)) "1.000000,1.000000,1.000000") "Undefined" "MultiplyWithRoot" 0 0)
  (Game|SpawnActorfromClass "/Game/GAME_Shooter/Folder_Charly/Chaos/PropsChaos/BP_box_bois.BP_box_bois_C" (Math|Transform|MakeTransform (Transformation|GetWorldLocation (Variables|Default|GetBox9)) (Math|Rotator|MakeRotator 0.0 0.0 (Math|Random|RandomFloatinRange 0.0 3.6e+02)) "1.000000,1.000000,1.000000") "Undefined" "MultiplyWithRoot" 0 0)
  (Game|SpawnActorfromClass "/Game/GAME_Shooter/Folder_Charly/Chaos/PropsChaos/BP_box_bois.BP_box_bois_C" (Math|Transform|MakeTransform (Transformation|GetWorldLocation (Variables|Default|GetBox10)) (Math|Rotator|MakeRotator 0.0 0.0 (Math|Random|RandomFloatinRange 0.0 3.6e+02)) "1.000000,1.000000,1.000000") "Undefined" "MultiplyWithRoot" 0 0)
  (Game|SpawnActorfromClass "/Game/GAME_Shooter/Folder_Charly/Chaos/PropsChaos/BP_box_bois.BP_box_bois_C" (Math|Transform|MakeTransform (Transformation|GetWorldLocation (Variables|Default|GetBox11)) (Math|Rotator|MakeRotator 0.0 0.0 (Math|Random|RandomFloatinRange 0.0 3.6e+02)) "1.000000,1.000000,1.000000") "Undefined" "MultiplyWithRoot" 0 0)
  (Game|SpawnActorfromClass "/Game/GAME_Shooter/Folder_Charly/Chaos/PropsChaos/BP_box_bois.BP_box_bois_C" (Math|Transform|MakeTransform (Transformation|GetWorldLocation (Variables|Default|GetBox12)) (Math|Rotator|MakeRotator 0.0 0.0 (Math|Random|RandomFloatinRange 0.0 3.6e+02)) "1.000000,1.000000,1.000000") "Undefined" "MultiplyWithRoot" 0 0)
  (Game|SpawnActorfromClass "/Game/GAME_Shooter/Folder_Charly/Chaos/PropsChaos/BP_box_bois.BP_box_bois_C" (Math|Transform|MakeTransform (Transformation|GetWorldLocation (Variables|Default|GetBox13)) (Math|Rotator|MakeRotator 0.0 0.0 (Math|Random|RandomFloatinRange 0.0 3.6e+02)) "1.000000,1.000000,1.000000") "Undefined" "MultiplyWithRoot" 0 0)
  (Game|SpawnActorfromClass "/Game/GAME_Shooter/Folder_Charly/Chaos/PropsChaos/BP_box_bois.BP_box_bois_C" (Math|Transform|MakeTransform (Transformation|GetWorldLocation (Variables|Default|GetBox14)) (Math|Rotator|MakeRotator 0.0 0.0 (Math|Random|RandomFloatinRange 0.0 3.6e+02)) "1.000000,1.000000,1.000000") "Undefined" "MultiplyWithRoot" 0 0)
  (Game|SpawnActorfromClass "/Game/GAME_Shooter/Folder_Charly/Chaos/PropsChaos/BP_box_bois.BP_box_bois_C" (Math|Transform|MakeTransform (Transformation|GetWorldLocation (Variables|Default|GetBox15)) (Math|Rotator|MakeRotator 0.0 0.0 (Math|Random|RandomFloatinRange 0.0 3.6e+02)) "1.000000,1.000000,1.000000") "Undefined" "MultiplyWithRoot" 0 0)
  (Game|SpawnActorfromClass "/Game/GAME_Shooter/Folder_Charly/Chaos/PropsChaos/BP_box_bois.BP_box_bois_C" (Math|Transform|MakeTransform (Transformation|GetWorldLocation (Variables|Default|GetBox16)) (Math|Rotator|MakeRotator 0.0 0.0 (Math|Random|RandomFloatinRange 0.0 3.6e+02)) "1.000000,1.000000,1.000000") "Undefined" "MultiplyWithRoot" 0 0))

(event Collision|EventActorBeginOverlap
  (params (OtherActor :type Actor%20Object%20Reference)))

(event EventTick
  (params (DeltaSeconds :type Float%20%28single-precision%29)))

(fn ConstructionScript
  (|CallParentFunction))