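; BP_Empty_Room2 is a room Blueprint in the casino game's procedural generation folder that fills itself with barrel props.
; On BeginPlay it runs the parent logic, then spawns four half-scale BP_tonneau actors at the world locations of its Tonneau marker components.
; The construction script only calls the parent, and the overlap and tick events are unused.
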(event EventBeginPlay
  (|CallParentFunction)
  (Game|SpawnActorfromClass "/Game/GAME_Shooter/Folder_Charly/Chaos/PropsChaos/BP_tonneau.BP_tonneau_C" (Math|Transform|MakeTransform (Transformation|GetWorldLocation (Variables|Default|GetTonneau)) "0, 0, 0" "0.500000,0.500000,0.500000") "Undefined" "MultiplyWithRoot" 0 0)
  (Game|SpawnActorfromClass "/Game/GAME_Shooter/Folder_Charly/Chaos/PropsChaos/BP_tonneau.BP_tonneau_C" (Math|Transform|MakeTransform (Transformation|GetWorldLocation (Variables|Default|GetTonneau1)) "0, 0, 0" "0.500000,0.500000,0.500000") "Undefined" "MultiplyWithRoot" 0 0)
  (Game|SpawnActorfromClass "/Game/GAME_Shooter/Folder_Charly/Chaos/PropsChaos/BP_tonneau.BP_tonneau_C" (Math|Transform|MakeTransform (Transformation|GetWorldLocation (Variables|Default|GetTonneau2)) "0, 0, 0" "0.500000,0.500000,0.500000") "Undefined" "MultiplyWithRoot" 0 0)
  (Game|SpawnActorfromClass "/Game/GAME_Shooter/Folder_Charly/Chaos/PropsChaos/BP_tonneau.BP_tonneau_C" (Math|Transform|MakeTransform (Transformation|GetWorldLocation (Variables|Default|GetTonneau3)) "0, 0, 0" "0.500000,0.500000,0.500000") "Undefined" "MultiplyWithRoot" 0 0))

(event Collision|EventActorBeginOverlap
  (params (OtherActor :type Actor%20Object%20Reference)))

(event EventTick
  (params (DeltaSeconds :type Float%20%28single-precision%29)))

(fn ConstructionScript
  (|CallParentFunction))