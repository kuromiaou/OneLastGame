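; Dungeon generator actor that clears existing rooms on BeginPlay and builds a new room layout by random walk on a grid.
; From a start room, it steps in four directions, spawning random room classes on free cells and linking neighbours through RoomConnection.
; Revisited cells only gain a connection without using the room budget.
; The final room is BP_LastRoom, where the player is teleported, then every room runs CreatePath.
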(event Custom|GenerateDungeon
  (Variables|Default|SetRoomLeft (Variables|Default|GetRoomAmount))
  (bind _returnvalue (Game|SpawnActorfromClass "/Game/GAME_Casino/Folder_Lorenzo/ProceduralGeneration/BP_StartRoom.BP_StartRoom_C" (Math|Transform|MakeTransform "0, 0, 0" "0, 0, 0" "1.000000,1.000000,1.000000") "Undefined" "MultiplyWithRoot" 0 0))
  (bind _output_get (Variables|Default|SetStartRoom _returnvalue))
  (Utilities|Map|Add (Variables|Default|GetRooms) _output_get (Math|Vector2D|MakeVector2D (.x (Transformation|GetActorLocation _returnvalue)) (.y (Transformation|GetActorLocation _returnvalue))))
  (Variables|Default|SetPreviousRoom (Variables|Default|GetStartRoom))
  (bind _result (Math|Integer|DecrementInt (Variables|Default|GetRoomLeft))
    (:%20%20
      (Variables|Default|SetRoomLeft _result)
      (if (> (Variables|Default|GetRoomLeft) 0) :!label _label
        (CallFunction|SpawnRandomRooom)
        (goto _label)
        (else
          (bind _keys (Utilities|Map|Keys (Variables|Default|GetRooms)))
          (for _array_element _keys
            (Default|CreatePath _array_element)
            (Variables|Default|SetDungeonGenerated true)))))))

(event Custom|ResetDungeon
  (bind _outactors (Actor|GetAllActorsOfClass "/Game/GAME_Casino/Folder_Lorenzo/ProceduralGeneration/BP_RoomParent.BP_RoomParent_C"))
  (for _array_element _outactors
    (Actor|DestroyActor _array_element)))

(event EventBeginPlay
  (CallFunction|ResetDungeon)
  (CallFunction|GenerateDungeon))

(fn ConstructionScript)

(fn SpawnRandomRooom
  (bind _rooms (Variables|Default|GetRooms))
  (bind _output_get (LocalVariables|SetPotentialLoc (Utilities|Select :Index (Math|Random|RandomIntegerinRange 0 3) :Option%200 (Math|Vector2D|MakeVector2D (+ (.X (Math|Vector2D|BreakVector2D (.Value (Utilities|Map|Find (Variables|Default|GetRooms) (Variables|Default|GetPreviousRoom))))) (.x (Variables|Default|GetGridSize))) (.Y (Math|Vector2D|BreakVector2D (.Value (Utilities|Map|Find (Variables|Default|GetRooms) (Variables|Default|GetPreviousRoom)))))) :Option%201 (Math|Vector2D|MakeVector2D (.X (Math|Vector2D|BreakVector2D (.Value (Utilities|Map|Find (Variables|Default|GetRooms) (Variables|Default|GetPreviousRoom))))) (+ (.Y (Math|Vector2D|BreakVector2D (.Value (Utilities|Map|Find (Variables|Default|GetRooms) (Variables|Default|GetPreviousRoom))))) (.y (Variables|Default|GetGridSize)))) :Option%202 (Math|Vector2D|MakeVector2D (- (.X (Math|Vector2D|BreakVector2D (.Value (Utilities|Map|Find (Variables|Default|GetRooms) (Variables|Default|GetPreviousRoom))))) (.x (Variables|Default|GetGridSize))) (.Y (Math|Vector2D|BreakVector2D (.Value (Utilities|Map|Find (Variables|Default|GetRooms) (Variables|Default|GetPreviousRoom)))))) :Option%203 (Math|Vector2D|MakeVector2D (.X (Math|Vector2D|BreakVector2D (.Value (Utilities|Map|Find (Variables|Default|GetRooms) (Variables|Default|GetPreviousRoom))))) (- (.Y (Math|Vector2D|BreakVector2D (.Value (Utilities|Map|Find (Variables|Default|GetRooms) (Variables|Default|GetPreviousRoom))))) (.y (Variables|Default|GetGridSize)))))))
  (bind _values (Utilities|Map|Values (Variables|Default|GetRooms)))
  (if (Utilities|Array|ContainsItem _values _output_get)
    (bind _values_2 (Utilities|Map|Values _rooms))
    (bind _keys (Utilities|Map|Keys _rooms))
    (LocalVariables|SetCurrentRoom (Utilities|Array|Get(acopy) _keys (Utilities|Array|FindItem _values_2 (LocalVariables|GetPotentialLoc))))
    (Utilities|Set|Add (Variables|/Game/GAME_Casino/Folder_Lorenzo/ProceduralGeneration/BP_RoomParent.BP_RoomParent_C|GetRoomConnection (LocalVariables|GetCurrentRoom)) (Variables|Default|GetPreviousRoom))
    (Utilities|Set|Add (Variables|/Game/GAME_Casino/Folder_Lorenzo/ProceduralGeneration/BP_RoomParent.BP_RoomParent_C|GetRoomConnection (Variables|Default|GetPreviousRoom)) (LocalVariables|GetCurrentRoom))
    (Variables|Default|SetPreviousRoom (LocalVariables|GetCurrentRoom))
    (else
      (if (<= (Variables|Default|GetRoomLeft) 1)
        (bind _returnvalue (Game|SpawnActorfromClass "/Game/GAME_Casino/Folder_Lorenzo/ProceduralGeneration/BP_LastRoom.BP_LastRoom_C" (Math|Transform|MakeTransform (Math|Vector|MakeVector (.X (Math|Vector2D|BreakVector2D (LocalVariables|GetPotentialLoc))) (.Y (Math|Vector2D|BreakVector2D (LocalVariables|GetPotentialLoc))) -2e+03) "0, 0, 0" "1.000000,1.000000,1.000000") "Undefined" "MultiplyWithRoot" 0 0))
        (Transformation|SetActorLocation (Game|GetPlayerCharacter 0) (Math|Vector|MakeVector (.x (Transformation|GetActorLocation _returnvalue)) (.y (Transformation|GetActorLocation _returnvalue)) (+ (.z (Transformation|GetActorLocation _returnvalue)) 5e+01)) false false)
        (bind _output_get_2 (LocalVariables|SetCurrentRoom _returnvalue))
        (Utilities|Map|Add (Variables|Default|GetRooms) _output_get_2 (Math|Vector2D|MakeVector2D (.x (Transformation|GetActorLocation _returnvalue)) (.y (Transformation|GetActorLocation _returnvalue))))
        (else
          (bind _returnvalue_2 (Game|SpawnActorfromClass (.OutItem (Utilities|Array|Random (Variables|Default|GetRandomRoom))) (Math|Transform|MakeTransform (Math|Vector|MakeVector (.X (Math|Vector2D|BreakVector2D (LocalVariables|GetPotentialLoc))) (.Y (Math|Vector2D|BreakVector2D (LocalVariables|GetPotentialLoc))) -2e+03) "0, 0, 0" "1.000000,1.000000,1.000000") "Undefined" "MultiplyWithRoot" 0 0))
          (bind _asbp_room_parent (Utilities|Casting|CastToBP_RoomParent _returnvalue_2))
          (Utilities|Array|Add (Variables|Default|GetRoomList) _asbp_room_parent)
          (bind _output_get_3 (LocalVariables|SetCurrentRoom _asbp_room_parent))
          (Utilities|Map|Add (Variables|Default|GetRooms) _output_get_3 (Math|Vector2D|MakeVector2D (.x (Transformation|GetActorLocation _asbp_room_parent)) (.y (Transformation|GetActorLocation _asbp_room_parent))))))
      (Math|Integer|DecrementInt (Variables|Default|GetRoomLeft)
        (:%20%20
          (Utilities|Set|Add (Variables|/Game/GAME_Casino/Folder_Lorenzo/ProceduralGeneration/BP_RoomParent.BP_RoomParent_C|GetRoomConnection (LocalVariables|GetCurrentRoom)) (Variables|Default|GetPreviousRoom))
          (Utilities|Set|Add (Variables|/Game/GAME_Casino/Folder_Lorenzo/ProceduralGeneration/BP_RoomParent.BP_RoomParent_C|GetRoomConnection (Variables|Default|GetPreviousRoom)) (LocalVariables|GetCurrentRoom))
          (Variables|Default|SetPreviousRoom (LocalVariables|GetCurrentRoom)))))))