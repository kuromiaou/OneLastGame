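; Base procedural-generation room for the casino game, with four walls that open toward connected rooms.
; BeginPlay stores its XY location as Coordinates and has a roughly 30% chance to spawn an actor at its Arrow component.
; CreatePath compares Coordinates with each room in RoomConnection to open the facing wall.
; RepNotify wall states toggle each wall's visibility and collision.
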(event Custom|CreatePath
  (bind _result (Utilities|Set|ToArray (Variables|Default|GetRoomConnection)))
  (for _array_element _result
    (if (!= (.x (Variables|BP_RoomParent_C|GetCoordinates _array_element)) (.x (Variables|Default|GetCoordinates)))
      (if (> (.x (Variables|BP_RoomParent_C|GetCoordinates _array_element)) (.x (Variables|Default|GetCoordinates)))
        (Variables|Default|SetTopWallState "NewEnumerator1")
        (else
          (Variables|Default|SetBottomWallState "NewEnumerator1")))
      (elif (> (.y (Variables|BP_RoomParent_C|GetCoordinates _array_element)) (.y (Variables|Default|GetCoordinates)))
        (Variables|Default|SetRightWallState "NewEnumerator1")
        (else
          (Variables|Default|SetLeftWallState "NewEnumerator1"))))))

(event EventBeginPlay
  (bind _returnvalue (Transformation|GetActorLocation))
  (if (>= (Math|Random|RandomFloatinRange 0.0 1e+02) 7e+01)
    (Game|SpawnActorfromClass "/Game/GAME_Shooter/Folder_Lucas/BP_SpawnerPortal_Lucas.BP_SpawnerPortal_Lucas_C" (Math|Transform|MakeTransform (.location (Transformation|GetWorldTransform (Variables|Default|GetArrow))) "0, 0, 0" "1.000000,1.000000,1.000000") "Undefined" "MultiplyWithRoot" 0 0))
  (Variables|Default|SetCoordinates (Math|Vector2D|MakeVector2D (.x _returnvalue) (.y _returnvalue))))

(fn ConstructionScript)

(fn OnRepTopWallState
  (bind _top (Variables|Default|GetTop))
  (bind _top_2 (Variables|Default|GetTop))
  (switch Utilities|FlowControl|Switch|SwitchonE_WallState (Variables|Default|GetTopWallState)
    (:NewEnumerator0
      (Rendering|SetVisibility _top_2 true false)
      (Collision|SetCollisionEnabled _top_2 "QueryAndPhysics"))
    (:NewEnumerator1
      (Rendering|SetVisibility _top false false)
      (Collision|SetCollisionEnabled _top "NoCollision"))))

(fn OnRepBottomWallState
  (bind _bottom (Variables|Default|GetBottom))
  (switch Utilities|FlowControl|Switch|SwitchonE_WallState (Variables|Default|GetBottomWallState)
    (:NewEnumerator0
      (Rendering|SetVisibility _bottom true false)
      (Collision|SetCollisionEnabled _bottom "QueryAndPhysics"))
    (:NewEnumerator1
      (Rendering|SetVisibility _bottom false false)
      (Collision|SetCollisionEnabled _bottom "NoCollision"))))

(fn OnRepRightWallState
  (bind _right (Variables|Default|GetRight))
  (switch Utilities|FlowControl|Switch|SwitchonE_WallState (Variables|Default|GetRightWallState)
    (:NewEnumerator0
      (Rendering|SetVisibility _right true false)
      (Collision|SetCollisionEnabled _right "QueryAndPhysics"))
    (:NewEnumerator1
      (Rendering|SetVisibility _right false false)
      (Collision|SetCollisionEnabled _right "NoCollision"))))

(fn OnRepLeftWallState
  (bind _left (Variables|Default|GetLeft))
  (switch Utilities|FlowControl|Switch|SwitchonE_WallState (Variables|Default|GetLeftWallState)
    (:NewEnumerator0
      (Rendering|SetVisibility _left true false)
      (Collision|SetCollisionEnabled _left "QueryAndPhysics"))
    (:NewEnumerator1
      (Rendering|SetVisibility _left false false)
      (Collision|SetCollisionEnabled _left "NoCollision"))))