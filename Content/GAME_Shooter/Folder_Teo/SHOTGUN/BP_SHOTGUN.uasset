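; Shotgun weapon Blueprint that fires a spread of bullets when its Shoot event runs for a given character.
; Shoot loops over the configured shot count, spawning a scaled-down BP_BULLET at the character's first-person camera with that character as owner.
; Each bullet gets its direction from the character's GetSprayAngle, using the camera's forward vector and the shotgun precision as maximum angle.
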(event EventShoot
  (params (Character :type BP%20First%20Person%20Character%20Object%20Reference))
  (bind _firstpersoncamera (Variables|/Game/FirstPerson/Blueprints/BP_FirstPersonCharacter.BP_FirstPersonCharacter_C|GetFirstPersonCamera Character))
  (for _index (range 0 (Variables|Default|Getshotgun/nb_shot))
    (Game|SpawnActorfromClass "/Game/GAME_Shooter/Folder_Teo/BP_BULLET.BP_BULLET_C" (Math|Transform|MakeTransform (Transformation|GetWorldLocation _firstpersoncamera) (Default|GetSprayAngle Character (Math|Vector|GetForwardVector (Transformation|GetWorldRotation _firstpersoncamera)) (Variables|Default|Getshotgun/precision)) "0.250000,0.250000,0.250000") "Undefined" "MultiplyWithRoot" Character 0)))

(fn ConstructionScript
  (|CallParentFunction))