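; BP_Lucas_ProjectileBoss is a boss projectile that damages the player on overlap and destroys itself after five seconds.
; On overlapping BP_FirstPersonCharacter, it looks up a BP_Lucas_BossDistance in the level and passes that boss's PlayerTakeDamage result to the player's AddStats.
; It then destroys itself, applying no damage if no such boss exists.
; Overlaps with other actors are ignored.
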(event EventBeginPlay
  (Utilities|FlowControl|Delay 5.0)
  (Actor|DestroyActor))

(event Collision|EventActorBeginOverlap
  (params (OtherActor :type Actor%20Object%20Reference))
  (bind _asbp_first_person_character (Utilities|Casting|CastToBP_FirstPersonCharacter OtherActor))
  (bind _outactors (Actor|GetAllActorsOfClass "/Game/GAME_Shooter/Folder_Lucas/BP_Lucas_BossDistance.BP_Lucas_BossDistance_C"))
  (if (!= (Utilities|Array|Length _outactors) 0)
    (bind _returnvalue (Actor|GetActorOfClass "/Game/GAME_Shooter/Folder_Lucas/BP_Lucas_BossDistance.BP_Lucas_BossDistance_C"))
    (bind _damages (Default|PlayerTakeDamage _returnvalue))
    (Default|AddStats _asbp_first_person_character "NewEnumerator0" _damages)
    (Actor|DestroyActor)
    (else
      (Actor|DestroyActor))))

(fn ConstructionScript)