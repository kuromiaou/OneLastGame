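; Enemy spawner portal that releases three timed waves on BeginPlay: melee (CAC) enemies, then distance enemies, then a distance boss, separated by short delays.
; Each wave has its own function that spawns actors at the portal's transform, spaced along world X by loop index, with the boss raised in Z.
; The loops run from zero through Number inclusive, so a non-zero count yields one extra enemy.
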(event EventBeginPlay
  (CallFunction|SpawnCAC 3)
  (Utilities|FlowControl|Delay 2.0)
  (CallFunction|SpawnDistance 1)
  (Utilities|FlowControl|Delay 2.0)
  (CallFunction|SpawnBoss 1))

(event Collision|EventActorBeginOverlap
  (params (OtherActor :type Actor%20Object%20Reference)))

(event EventTick
  (params (DeltaSeconds :type Float%20%28single-precision%29)))

(fn ConstructionScript)

(fn SpawnCAC
  (params (Number :type Integer))
  (bind _self self)
  (bind _returnvalue (Transformation|GetActorTransform _self))
  (bind (_location _rotation _scale) (Math|Transform|BreakTransform _returnvalue))
  (bind (_x _y _z) (Math|Vector|BreakVector _location))
  (if (!= Number 0)
    (for _index (range 0 Number)
      (Game|SpawnActorfromClass "/Game/GAME_Shooter/Folder_Lucas/BP_Lucas_CACEnemy.BP_Lucas_CACEnemy_C" (Math|Transform|MakeTransform (Math|Vector|MakeVector (+ (* _index 50) _x) _y _z) _rotation _scale) "Undefined" "MultiplyWithRoot" 0 0))))

(fn SpawnDistance
  (params (Number :type Integer))
  (bind _self self)
  (bind _returnvalue (Transformation|GetActorTransform _self))
  (bind (_location _rotation _scale) (Math|Transform|BreakTransform _returnvalue))
  (bind (_x _y _z) (Math|Vector|BreakVector _location))
  (if (!= Number 0)
    (for _index (range 0 Number)
      (Game|SpawnActorfromClass "/Game/GAME_Shooter/Folder_Lucas/BP_Lucas_DistanceEnemy.BP_Lucas_DistanceEnemy_C" (Math|Transform|MakeTransform (Math|Vector|MakeVector (+ (* _index 50) _x) _y _z) _rotation _scale) "Undefined" "MultiplyWithRoot" 0 0))))

(fn SpawnBoss
  (params (number :type Integer))
  (bind _self self)
  (bind _returnvalue (Transformation|GetActorTransform _self))
  (bind (_location _rotation _scale) (Math|Transform|BreakTransform _returnvalue))
  (bind (_x _y _z) (Math|Vector|BreakVector _location))
  (if (!= number 0)
    (for _index (range 0 number)
      (Game|SpawnActorfromClass "/Game/GAME_Shooter/Folder_Lucas/BP_Lucas_BossDistance.BP_Lucas_BossDistance_C" (Math|Transform|MakeTransform (Math|Vector|MakeVector (+ (* _index 50) _x) _y (+ _z 1e+02)) _rotation _scale) "Undefined" "MultiplyWithRoot" 0 0))))