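; BP_Lucas_BossDistance is a shootable boss actor that keeps its stats, such as HP and Damage, in an enum-keyed map.
; When a BP_BULLET overlaps it, it subtracts the first-person player's Damage stat from its HP, and Tick destroys it once HP reaches zero.
; Helper functions read and add to stats, and PlayerTakeDamage returns the boss's negated Damage.
; No movement or ranged-attack logic is implemented here.
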(event EventBeginPlay
  (|CallParentFunction) ; This node is disabled and will not be called.\nDrag off pins to build functionality.
)

(event Collision|EventActorBeginOverlap
  (params (OtherActor :type Actor%20Object%20Reference))
  (Utilities|Casting|CastToBP_BULLET OtherActor)
  (bind _asbp_first_person_character (Utilities|Casting|CastToBP_FirstPersonCharacter (Game|GetPlayerCharacter 0)))
  (bind _value (Default|GetStats _asbp_first_person_character "NewEnumerator10"))
  (CallFunction|AddStats "NewEnumerator0" (* _value -1.0))
  (Development|PrintString (Utilities|String|ToString(Float) (.Value (Utilities|Map|Find (Variables|Default|GetEnum) "NewEnumerator0")))))

(event EventTick
  (params (DeltaSeconds :type Float%20%28single-precision%29))
  (if (<= (.Value (Utilities|Map|Find (Variables|Default|GetEnum) "NewEnumerator0")) 0.0)
    (Actor|DestroyActor)))

(fn ConstructionScript
  (|CallParentFunction))

(fn GetStats
  (params (Key :type E_Stats%20Enum :default "NewEnumerator0"))
  (return (.Value (Utilities|Map|Find (Variables|Default|GetEnum) Key))))

(fn PlayerTakeDamage
  (bind _enum (Variables|Default|GetEnum))
  (bind _value (Utilities|Map|Find _enum "NewEnumerator10"))
  (bind _returnvalue (* _value -1.0))
  (Development|PrintText (Utilities|Text|ToText(Float) _returnvalue "HalfToEven"))
  (return _returnvalue))

(fn AddStats
  (params (key :type E_Stats%20Enum :default "NewEnumerator0") (value :type Float%20%28double-precision%29))
  (bind _enum (Variables|Default|GetEnum))
  (Utilities|Map|Add _enum key (+ value (.Value (Utilities|Map|Find _enum key))))
  (switch Utilities|FlowControl|Switch|SwitchonE_Stats key))