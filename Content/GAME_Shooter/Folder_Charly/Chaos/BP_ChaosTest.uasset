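; Chaos destruction test actor that swaps itself for a breakable geometry collection when it is hit.
; On Hit it prints a debug message, spawns a GeometryCollectionActor at its own transform, assigns the GeometryCollection asset as rest collection, then destroys itself.
; BeginPlay caches the Cube's static mesh, though nothing reads it, and an IsBroken check is left unconnected.
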(event EventBeginPlay
  (Variables|Default|SetstaticMesh (Variables|/Script/Engine.StaticMeshComponent|GetStaticMesh (Variables|Default|GetCube))))

(event Collision|EventHit
  (params (MyComp :type Primitive%20Component%20Object%20Reference) (Other :type Actor%20Object%20Reference) (OtherComp :type Primitive%20Component%20Object%20Reference) (bSelfMoved :type Boolean) (HitLocation :type Vector :default "0, 0, 0") (HitNormal :type Vector :default "0, 0, 0") (NormalImpulse :type Vector :default "0, 0, 0") (Hit :type Hit%20Result%20Structure%20%28by%20ref%29))
  (Development|PrintText "Hello")
  (bind _returnvalue (Game|SpawnActorfromClass "/Script/GeometryCollectionEngine.GeometryCollectionActor" (Transformation|GetActorTransform) "Undefined" "MultiplyWithRoot" 0 0))
  (Class|GeometryCollectionComponent|SetRestCollection (Variables|/Script/GeometryCollectionEngine.GeometryCollectionActor|GetGeometryCollectionComponent _returnvalue) (Variables|Default|GetGeometryCollection) true)
  (Actor|DestroyActor))

(fn ConstructionScript)