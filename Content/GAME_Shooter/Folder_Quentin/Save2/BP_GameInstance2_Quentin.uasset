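; Game instance Blueprint for the shooter that saves and loads player progress through BP_SaveGame2_Quentin slots.
; Saving requires a valid current save, then replaces it with a new object holding a struct of the character's transform and enum-indexed stats.
; Loading reads the slot or creates an empty save.
; Applying restores only the transform, read from PlayerTransform rather than the saved PlayerData struct.
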(fn SaveGametoSlot
  (params (SlotName :type String))
  (Utilities|IsValid (Variables|Default|GetCurrentSaveGame)
    (:Is%20Valid
      (bind _returnvalue (SaveGame|CreateSaveGameObject "/Game/GAME_Shooter/Folder_Quentin/Save2/BP_SaveGame2_Quentin.BP_SaveGame2_Quentin_C"))
      (Development|PrintString "Creation Save")
      (bind _output_get (Variables|Default|SetCurrentSaveGame _returnvalue))
      (bind _stc (CallFunction|SaveVariablesFCTN))
      (Variables|/Game/GAME_Shooter/Folder_Quentin/Save2/BP_SaveGame2_Quentin.BP_SaveGame2_Quentin_C|SetPlayerData _output_get _stc)
      (SaveGame|SaveGametoSlot _output_get SlotName))))

(fn MyLoadGame
  (params (SlotName :type String))
  (bind _returnvalue (SaveGame|DoesSaveGameExist SlotName))
  (if _returnvalue
    (bind _returnvalue_2 (SaveGame|LoadGamefromSlot SlotName))
    (bind _asbp_save_game_2_quentin (Utilities|Casting|CastToBP_SaveGame2_Quentin _returnvalue_2))
    (Variables|Default|SetCurrentSaveGame _asbp_save_game_2_quentin)
    (else
      (bind _returnvalue_3 (SaveGame|CreateSaveGameObject "/Game/GAME_Shooter/Folder_Quentin/Save2/BP_SaveGame2_Quentin.BP_SaveGame2_Quentin_C"))
      (Variables|Default|SetCurrentSaveGame _returnvalue_3))))

(fn ApplyLoadedDatatoPlayer
  (bind _currentsavegame (Variables|Default|GetCurrentSaveGame))
  (Utilities|IsValid _currentsavegame
    (:Is%20Valid
      (Transformation|SetActorTransform (Game|GetPlayerCharacter 0) (Variables|/Game/GAME_Shooter/Folder_Quentin/Save2/BP_SaveGame2_Quentin.BP_SaveGame2_Quentin_C|GetPlayerTransform _currentsavegame)))))

(fn SaveVariablesFCTN
  (Utilities|Casting|CastToBP_GameInstance_Quentin (Game|GetGameInstance))
  (bind _asbp_first_person_character_child_quentin (Utilities|Casting|CastToBP_FirstPersonCharacter_Child_Quentin (Game|GetPlayerCharacter 0)))
  (bind _value (Default|GetStats _asbp_first_person_character_child_quentin "NewEnumerator0"))
  (bind _value_2 (Default|GetStats _asbp_first_person_character_child_quentin "NewEnumerator1"))
  (bind _value_3 (Default|GetStats _asbp_first_person_character_child_quentin "NewEnumerator2"))
  (bind _value_4 (Default|GetStats _asbp_first_person_character_child_quentin "NewEnumerator3"))
  (bind _value_5 (Default|GetStats _asbp_first_person_character_child_quentin "NewEnumerator4"))
  (bind _value_6 (Default|GetStats _asbp_first_person_character_child_quentin "NewEnumerator5"))
  (bind _value_7 (Default|GetStats _asbp_first_person_character_child_quentin "NewEnumerator6"))
  (bind _value_8 (Default|GetStats _asbp_first_person_character_child_quentin "NewEnumerator7"))
  (bind _value_9 (Default|GetStats _asbp_first_person_character_child_quentin "NewEnumerator8"))
  (bind _value_10 (Default|GetStats _asbp_first_person_character_child_quentin "NewEnumerator9"))
  (bind _value_11 (Default|GetStats _asbp_first_person_character_child_quentin "NewEnumerator10"))
  (bind _value_12 (Default|GetStats _asbp_first_person_character_child_quentin "NewEnumerator11"))
  (bind _value_13 (Default|GetStats _asbp_first_person_character_child_quentin "NewEnumerator12"))
  (bind _value_14 (Default|GetStats _asbp_first_person_character_child_quentin "NewEnumerator13"))
  (bind _value_15 (Default|GetStats _asbp_first_person_character_child_quentin "NewEnumerator14"))
  (bind _value_16 (Default|GetStats _asbp_first_person_character_child_quentin "NewEnumerator15"))
  (bind _value_17 (Default|GetStats _asbp_first_person_character_child_quentin "NewEnumerator16"))
  (bind _value_18 (Default|GetStats _asbp_first_person_character_child_quentin "NewEnumerator17"))
  (bind _value_19 (Default|GetStats _asbp_first_person_character_child_quentin "NewEnumerator18"))
  (return (Utilities|Struct|MakeSTC_SaveGame_Quentin (Transformation|GetActorTransform _asbp_first_person_character_child_quentin) _value _value_2 _value_3 _value_4 _value_5 _value_6 _value_7 _value_8 _value_9 _value_10 _value_11 0.0 _value_12 _value_13 0.0 _value_14 _value_15 _value_16 _value_17 _value_18 _value_19)))