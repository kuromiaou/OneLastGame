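; RPG rocket launcher weapon Blueprint that extends a parent weapon class and initializes its damage stats.
; On BeginPlay it runs the parent logic, sets its weapon ID, then picks a base damage that rises with rarity.
; It then adds DMGROKET to one entry of the current-stats map and writes the sum back.
; The rarity-based RPGBaseDmg does not feed that sum in this Blueprint.
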(event EventBeginPlay
  (|CallParentFunction)
  (Variables|Default|SetVAR_Weapon_ID 0)
  (CallFunction|FRPGRarityDmg)
  (CallFunction|FRPGWeaponDMG))

(event Collision|EventActorBeginOverlap
  (params (OtherActor :type Actor%20Object%20Reference))
  (|CallParentFunction OtherActor) ; Ce nœud est désactivé et ne sera pas appelé.\nFaites glisser les broches pour générer des fonctionnalités.
)

(event EventTick
  (params (DeltaSeconds :type Float%20%28single-precision%29))
  (|CallParentFunction DeltaSeconds) ; Ce nœud est désactivé et ne sera pas appelé.\nFaites glisser les broches pour générer des fonctionnalités.
)

(fn ConstructionScript
  (|CallParentFunction))

(fn FRPGWeaponDMG
  (bind _enum_weapons_current_stats (Variables|Default|GetENUM_Weapons_Current_Stats))
  (bind _output_get (Variables|Default|SetDMG%20ROKET (+ (Variables|Default|GetDMG%20ROKET) (.Value (Utilities|Map|Find _enum_weapons_current_stats "NewEnumerator10")))))
  (Utilities|Map|Add _enum_weapons_current_stats "NewEnumerator10" _output_get)
  (return))

(fn FRPGRarityDmg
  (switch Utilities|FlowControl|Switch|SwitchonE_Rarity (Variables|Default|GetENUM_Weapon_Current_Rarity)
    (:NewEnumerator0
      (Variables|Default|SetRPG_Base_Dmg 1e+01))
    (:NewEnumerator1
      (Variables|Default|SetRPG_Base_Dmg 2e+01))
    (:NewEnumerator2
      (Variables|Default|SetRPG_Base_Dmg 3e+01))
    (:NewEnumerator3
      (Variables|Default|SetRPG_Base_Dmg 4e+01))
    (:NewEnumerator4
      (Variables|Default|SetRPG_Base_Dmg 5e+01))
    (:NewEnumerator6
      (Variables|Default|SetRPG_Base_Dmg 6e+01))))

(fn NewFunction)