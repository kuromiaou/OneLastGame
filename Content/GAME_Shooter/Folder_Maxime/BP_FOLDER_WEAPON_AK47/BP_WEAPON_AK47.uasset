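; AK47 weapon Blueprint for the shooter, extending a parent weapon class with its own damage, shooting and reload logic.
; On BeginPlay it derives base damage from rarity and adds a bonus from the current-stats map.
; Shoot spawns BP_BULLET at the Arrow's transform.
; Tick polls Reload, which refills the magazine after a stat-scaled delay when NeedReload is set; the empty-magazine check is never called here.
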(event Custom|Reload
  (bind _enum_weapons_current_stats (Variables|Default|GetENUM_Weapons_Current_Stats))
  (if (Variables|Default|GetNeedReload)
    (Utilities|FlowControl|Delay (* 4.0 (.Value (Utilities|Map|Find _enum_weapons_current_stats "NewEnumerator7"))))
    (Variables|Default|SetVAR_MAG_AK47 (Class|KismetMathLibrary|ToInt64(Float) (.Value (Utilities|Map|Find _enum_weapons_current_stats "NewEnumerator19"))))))

(event EventBeginPlay
  (|CallParentFunction)
  (CallFunction|FAK47RarityDmg)
  (CallFunction|FAK47WeaponDMG))

(event Collision|EventActorBeginOverlap
  (params (OtherActor :type Actor%20Object%20Reference))
  (|CallParentFunction OtherActor) ; Ce nœud est désactivé et ne sera pas appelé.\nFaites glisser les broches pour générer des fonctionnalités.
)

(event EventTick
  (params (DeltaSeconds :type Float%20%28single-precision%29))
  (|CallParentFunction DeltaSeconds)
  (CallFunction|Reload))

(event EventShoot
  (params (Character :type BP%20First%20Person%20Character%20Object%20Reference))
  (CallFunction|FAK47Shoot))

(fn ConstructionScript
  (|CallParentFunction))

(fn FAK47RarityDmg
  (switch Utilities|FlowControl|Switch|SwitchonE_Rarity (Variables|Default|GetENUM_Weapon_Current_Rarity)
    (:NewEnumerator0
      (Variables|Default|SetAK47_Base_Dmg 1e+01))
    (:NewEnumerator1
      (Variables|Default|SetAK47_Base_Dmg 2e+01))
    (:NewEnumerator2
      (Variables|Default|SetAK47_Base_Dmg 3e+01))
    (:NewEnumerator3
      (Variables|Default|SetAK47_Base_Dmg 4e+01))
    (:NewEnumerator4
      (Variables|Default|SetAK47_Base_Dmg 5e+01))
    (:NewEnumerator6
      (Variables|Default|SetAK47_Base_Dmg 6e+01)))
  (return))

(fn FAK47WeaponDMG
  (Variables|Default|SetDMG_AK47 (+ (Variables|Default|GetAK47_Base_Dmg) (.Value (Utilities|Map|Find (Variables|Default|GetENUM_Weapons_Current_Stats) "NewEnumerator10")))))

(fn FAK47NeedReload?
  (if (== (Variables|Default|GetVAR_MAG_AK47) 0)
    (Variables|Default|SetNeedReload true)
    (return true)
    (else
      (return false))))

(fn FAK47Shoot
  (Game|SpawnActorfromClass "/Game/GAME_Shooter/Folder_Teo/BP_BULLET.BP_BULLET_C" (Transformation|GetWorldTransform (Variables|Default|GetArrow)) "AlwaysSpawn" "MultiplyWithRoot" 0 0))