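; Knife weapon Blueprint that extends a parent class and implements a timed attack through the Shoot event.
; Box starts inactive; when CanShoot is true, Shoot activates it for a short window, then deactivates it.
; CanShoot turns false only after that window closes and resets after a Delay-based cooldown.
; The Box overlap handler is empty, so this graph applies no hit effect or damage.
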(event OnComponentBeginOverlap(Box)
  (params (OverlappedComponent :type Primitive%20Component%20Object%20Reference) (OtherActor :type Actor%20Object%20Reference) (OtherComp :type Primitive%20Component%20Object%20Reference) (OtherBodyIndex :type Integer) (bFromSweep :type Boolean) (SweepResult :type Hit%20Result%20Structure%20%28by%20ref%29)))

(event EventBeginPlay
  (|CallParentFunction)
  (Components|Activation|SetActive (Variables|Default|GetBox) false false))

(event Collision|EventActorBeginOverlap
  (params (OtherActor :type Actor%20Object%20Reference))
  (|CallParentFunction OtherActor) ; Ce nœud est désactivé et ne sera pas appelé.\nFaites glisser les broches pour générer des fonctionnalités.
)

(event EventTick
  (params (DeltaSeconds :type Float%20%28single-precision%29))
  (|CallParentFunction DeltaSeconds) ; Ce nœud est désactivé et ne sera pas appelé.\nFaites glisser les broches pour générer des fonctionnalités.
)

(event EventShoot
  (params (Character :type BP%20First%20Person%20Character%20Object%20Reference))
  (bind _box (Variables|Default|GetBox))
  (if (Variables|Default|GetCanShoot?)
    (Components|Activation|SetActive _box true false)
    (Utilities|FlowControl|Delay 0.2)
    (Components|Activation|SetActive _box false false)
    (Variables|Default|SetCanShoot? false)
    (Utilities|FlowControl|Delay 2.0)
    (Variables|Default|SetCanShoot? true)))

(fn ConstructionScript
  (|CallParentFunction))